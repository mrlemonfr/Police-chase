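; bp_slideplatform is a sliding platform actor that moves its mesh along the vertical axis.
; Each Tick it adds a Z offset to the Platformmesh relative location, scaled by Speed and delta time, until that Z exceeds Distince2.
; Movement is one-way with no reset or reversal, and the construction script only calls its parent.
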(event EventTick
  (params (DeltaSeconds :type Float%20%28single-precision%29))
  (|CallParentFunction DeltaSeconds)
  (if (not (> (.z (Variables|/Script/Engine.SceneComponent|GetRelativeLocation (Variables|Default|Getplatformmesh))) (Variables|Default|Getdistince_2)))
    (Transformation|AddRelativeLocation (Variables|Default|Getplatformmesh) (Math|Vector|MakeVector 0.0 0.0 (* DeltaSeconds (Variables|Default|Getspeed))) false false)))

(fn ConstructionScript
  (|CallParentFunction))